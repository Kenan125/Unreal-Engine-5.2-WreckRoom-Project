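; BP_bullet is a short-lived projectile actor that lights up in a random color.
; On BeginPlay it adds a point light component, tints it from a random unit vector, and destroys itself after a three-second delay.
; A Launch function applies a forward velocity-change impulse to the static mesh, but the call to it in this event graph is disconnected.
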(event EventBeginPlay
  (bind _returnvalue (AddComponent|AddPointLightComponent false))
  (Rendering|Components|Light|SetLightColor _returnvalue (Math|Conversions|ToLinearColor(Vector) (Math|Random|RandomUnitVector)) true)
  (Utilities|FlowControl|Delay 3.0)
  (Actor|DestroyActor))

(event Collision|EventActorBeginOverlap
  (params (OtherActor :type Actor%20Object%20Reference)))

(event EventTick
  (params (DeltaSeconds :type Float%20%28single-precision%29)))

(fn ConstructionScript)

(fn Launch
  (Physics|AddImpulse (Variables|Debug|GetStaticMeshComponent) (* (Transformation|GetActorForwardVector) 2e+03) "None" true))